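; Lobby portal Blueprint that sends the player to Chapter 1 when their pawn enters its box trigger.
; On BeginPlay the box collision stays disabled for a short delay before switching to query-only.
; A player overlap disables the box to prevent retriggering, then asks the game state subsystem to travel to the Chapter1 state with a loading widget.
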(event OnComponentBeginOverlap(Box)
  (params (OverlappedComponent :type Primitive%20Component%20Object%20Reference) (OtherActor :type Actor%20Object%20Reference) (OtherComp :type Primitive%20Component%20Object%20Reference) (OtherBodyIndex :type Integer) (bFromSweep :type Boolean) (SweepResult :type Hit%20Result%20Structure%20%28by%20ref%29))
  (if (== OtherActor (Game|Player|GetPlayerPawn 0))
    (Collision|SetCollisionEnabled (Variables|Default|GetBox) "NoCollision")
    (Class|GameStateSubsystem|TraveltoState (Subsystems|GetGameStateSubsystem) "Chapter1" true)))

(event OnComponentEndOverlap(Box)
  (params (OverlappedComponent :type Primitive%20Component%20Object%20Reference) (OtherActor :type Actor%20Object%20Reference) (OtherComp :type Primitive%20Component%20Object%20Reference) (OtherBodyIndex :type Integer)))

(event EventBeginPlay
  (Collision|SetCollisionEnabled (Variables|Default|GetBox) "NoCollision")
  (Utilities|FlowControl|Delay 0.5)
  (Collision|SetCollisionEnabled (Variables|Default|GetBox) "QueryOnly"))

(fn ConstructionScript)